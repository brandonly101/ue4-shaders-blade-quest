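; Player character Blueprint with mouse-look and movement axes, jumping, a sword attack and a toggleable first/third-person view.
; Creates the PlayerHUD widget on BeginPlay and copies Health and Stamina into it every Tick.
; Sword collider overlaps deal damage during an attack, gated by IsAttacking, DealtDamage and CanDamage.
; F flip-flops cameras and mesh visibility, re-attaching the sword to the visible mesh's WEAPON socket.
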(event `self.ReceiveBeginPlay`
  ;[1 1 1] Initialize HUD
  (bind _returnvalue (`|CreateWidget` "/Game/Blueprints/PlayerHUD.PlayerHUD_C" (`GameplayStatics.GetPlayerController` 0)))
  (bind _output_get (set `self.PlayerHUD` _returnvalue))
  (set `/Game/Blueprints/PlayerHUD.HealthValue` (`self.Health`) _output_get)
  (set `/Game/Blueprints/PlayerHUD.StaminaValue` (`self.Stamina`) _output_get)
  (`UserWidget.AddToViewport` _output_get 0))

(event `InputAxis|AxisLookY`
  (params (AxisValue :type "Float (single-precision)"))
  ;[1 1 1] Player Movement Control and Actions
  (`self.AddControllerPitchInput` AxisValue))

(event `InputAxis|AxisLookX`
  (params (AxisValue :type "Float (single-precision)"))
  ;[1 1 1] Player Movement Control and Actions
  (`self.AddControllerYawInput` AxisValue))

(event `InputAxis|AxisMoveX`
  (params (AxisValue :type "Float (single-precision)"))
  ;[1 1 1] Player Movement Control and Actions
  (`self.AddMovementInput` (`self.GetActorRightVector`) AxisValue))

(event `self.ReceiveTick`
  (params (DeltaSeconds :type "Float (single-precision)"))
  (bind _playerhud (`self.PlayerHUD`))
  ;[1 1 1] Update HUD
  (`parent.ReceiveTick` DeltaSeconds)
  (set `/Game/Blueprints/PlayerHUD.HealthValue` (`self.Health`) _playerhud)
  (set `/Game/Blueprints/PlayerHUD.StaminaValue` (`self.Stamina`) _playerhud))

(event `InputAxis|AxisMoveY`
  (params (AxisValue :type "Float (single-precision)"))
  ;[1 1 1] Player Movement Control and Actions
  (`self.AddMovementInput` (`self.GetActorForwardVector`) AxisValue))

(event `InputAction|Jump`
  ;[1 1 1] Player Movement Control and Actions
  (:`Pressed`
    (`self.Jump`))
  (:`Released`
    (`self.StopJumping`)))

(event `InputAction|Attack`
  ;[1 1 1] Attacking Logic
  (:`Pressed`
    (if (not (`self.isAttacking`))
      (`self.Attack`))))

(event `self.SwordCollider.OnComponentBeginOverlap`
  (params (OtherActor :type "Actor Object Reference") (OtherComp :type "PrimitiveComponent Object Reference") (OtherBodyIndex :type Integer) (bFromSweep :type Boolean) (SweepResult :type "HitResult Structure (by ref)"))
  ;[1 1 1] Attacking Logic
  (if (and (`self.isAttacking`) (not (`self.dealtDamage`)) (!= OtherActor self) (`self.canDamage`))
    (`GameplayStatics.ApplyDamage` OtherActor (`self.Damage`) (`GameplayStatics.GetPlayerController` 0))
    (set `self.dealtDamage` true)))

(event `Key|F`
  ;[1 1 1] Toggle First-person/Third-person View
  (:`Pressed`
    (`/Engine/EditorBlueprintResources/StandardMacros.FlipFlop`
      (:`A`
        (`SceneComponent.K2_AttachTo` (`self.Sword`) (`self.Mesh3rdPerson`) "WEAPON" "KeepRelativeOffset" true)
        (`SceneComponent.SetHiddenInGame` (`self.Mesh`) true false)
        (`SceneComponent.SetHiddenInGame` (`self.Mesh3rdPerson`) false false)
        (`ActorComponent.Activate` (`self.Socket3rdPerson`) false)
        (`ActorComponent.Activate` (`self.Camera3rdPerson`) false)
        (`ActorComponent.Deactivate` (`self.Camera`)))
      (:`B`
        (`SceneComponent.K2_AttachTo` (`self.Sword`) (`self.Mesh`) "WEAPON" "KeepRelativeOffset" true)
        (`SceneComponent.SetHiddenInGame` (`self.Mesh3rdPerson`) true false)
        (`SceneComponent.SetHiddenInGame` (`self.Mesh`) false false)
        (`ActorComponent.Activate` (`self.Camera`) false)
        (`ActorComponent.Deactivate` (`self.Socket3rdPerson`))
        (`ActorComponent.Deactivate` (`self.Camera3rdPerson`))))))

(fn `UserConstructionScript`
  (`SceneComponent.K2_AttachTo` (`self.Mesh`) (`self.Camera`) "Root" "KeepRelativeOffset" true)
  (`SceneComponent.K2_AttachTo` (`self.Sword`) (`self.Mesh`) "WEAPON" "KeepRelativeOffset" true))