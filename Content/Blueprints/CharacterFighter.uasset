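; CharacterFighter is a fighter character Blueprint that manages health, stamina, damage taken and attack timing.
; Tick adds per-frame regen to health and stamina up to about 1.0, without delta-time scaling.
; Damage lowers health, pauses its regen briefly and clears IsAlive at zero.
; Attack spends stamina, enables its regen and uses speed-scaled delays to time the CanDamage window and cooldown, with no hit detection here.
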(event `self.ReceiveBeginPlay`)

(event `self.ReceiveActorBeginOverlap`
  (params (OtherActor :type "Actor Object Reference")))

(event `self.ReceiveTick`
  (params (DeltaSeconds :type "Float (single-precision)"))
  ;[1 1 1] Regeneration
  (`|ExecutionSequence`
    (:`then_0`
      (if (and (`self.RegenToggleHealth`) (<= (`self.Health`) 1.0))
        (set `self.Health` (+ (`self.Health`) (`self.HealthRegen`)))))
    (:`then_1`
      (if (and (`self.RegenToggleStamina`) (<= (`self.Stamina`) 1.0))
        (set `self.Stamina` (+ (`self.Stamina`) (`self.StaminaRegen`)))))))

(event `self.ReceiveAnyDamage`
  (params (Damage :type "Float (single-precision)") (DamageType :type "DamageType Object Reference") (InstigatedBy :type "Controller Object Reference") (DamageCauser :type "Actor Object Reference"))
  ;[1 1 1] Take Damage Logic
  (`|ExecutionSequence`
    (:`then_0`
      (set `self.Health` (- (`self.Health`) Damage)))
    (:`then_1`
      (set `self.RegenToggleHealth` false)
      (`KismetSystemLibrary.Delay` 1.0)
      (set `self.RegenToggleHealth` true))
    (:`then_2`
      (if (<= (`self.Health`) 0.0)
        (set `self.isAlive` false)))))

(event `Attack`
  ;[1 1 1] Attack Logic
  (`|ExecutionSequence`
    (:`then_0`
      (set `self.isAttacking` true)
      (set `self.dealtDamage` false)
      (set `self.canDamage` true)
      (`KismetSystemLibrary.Delay` (/ (`self.SpeedAttackAnim`) (`self.SpeedAttack`)))
      (set `self.canDamage` false)
      (`KismetSystemLibrary.Delay` (/ (`self.SpeedAttackAnimCD`) (`self.SpeedAttack`)))
      (set `self.isAttacking` false)
      (set `self.dealtDamage` false)
      (set `self.canDamage` false))
    (:`then_1`
      (set `self.RegenToggleStamina` true))
    (:`then_2`
      (set `self.Stamina` (- (`self.Stamina`) (`self.StaminaAttackUsage`))))))

(fn `UserConstructionScript`)