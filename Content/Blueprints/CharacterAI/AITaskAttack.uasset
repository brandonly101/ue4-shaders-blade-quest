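; Behavior Tree task that makes an AI-controlled CharacterFighter perform an attack.
; It caches the CharacterAIController on first execution, then calls Attack on the controlled fighter.
; Two delays, the attack animation and its cooldown, each scaled by attack speed, hold the task until it finishes successfully.
; A failed cast stops the flow without finishing the task.
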(event `self.ReceiveExecute`
  (params (OwnerActor :type "Actor Object Reference"))
  (if (not (!= (`self.AIControllerRef`) null))
    (bind _ascharacter_aicontroller (cast `/Game/Blueprints/CharacterAI/CharacterAIController` OwnerActor))
    (set `self.AIControllerRef` _ascharacter_aicontroller))
  (bind _ascharacter_fighter (cast `/Game/Blueprints/CharacterFighter` (`Controller.K2_GetPawn` (`self.AIControllerRef`))))
  ;[1 1 1] Attacking Logic
  (`/Game/Blueprints/CharacterFighter.Attack` _ascharacter_fighter)
  (`KismetSystemLibrary.Delay` (/ (`/Game/Blueprints/CharacterFighter.SpeedAttackAnim` _ascharacter_fighter) (`/Game/Blueprints/CharacterFighter.SpeedAttack` _ascharacter_fighter)))
  (`KismetSystemLibrary.Delay` (/ (`/Game/Blueprints/CharacterFighter.SpeedAttackAnimCD` _ascharacter_fighter) (`/Game/Blueprints/CharacterFighter.SpeedAttack` _ascharacter_fighter)))
  (`self.FinishExecute` true))