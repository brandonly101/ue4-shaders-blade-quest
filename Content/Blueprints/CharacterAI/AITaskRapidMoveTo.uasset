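; AITaskRapidMoveTo is a behavior tree task that moves an AI-controlled character toward a target actor.
; On execute it casts the owner to CharacterAIController and caches that reference for later runs.
; It runs AIMoveTo on the controlled pawn toward the AITarget blackboard actor, using CharacterRange as the acceptance radius.
; The task finishes successfully when the move succeeds; neither a failed move nor a failed cast calls FinishExecute.
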(event `self.ReceiveExecute`
  (params (OwnerActor :type "Actor Object Reference"))
  (if (not (!= (`self.AIControllerRef`) null))
    (bind _ascharacter_aicontroller (cast `/Game/Blueprints/CharacterAI/CharacterAIController` OwnerActor))
    (set `self.AIControllerRef` _ascharacter_aicontroller))
  (`|AIMoveTo` (`Controller.K2_GetPawn` (`self.AIControllerRef`)) (0.0 0.0 0.0) (`BTFunctionLibrary.GetBlackboardValueAsActor` (`self.AITarget`)) (`self.CharacterRange`)
    (:`OnSuccess`
      (`self.FinishExecute` true))))