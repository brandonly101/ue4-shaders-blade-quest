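; Behavior Tree service that handles aggro detection for CharacterAI, writing a visible target to the Blackboard.
; Each tick it sphere-traces around the controlled pawn for desired object types, ignoring all CharacterAI actors, then line-traces to each hit on the Camera channel.
; A clear line sets target actor and location, while a blocked one clears only the actor.
; The last hit processed wins, and no hits leaves both values unchanged.
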(event `self.ReceiveTick`
  (params (OwnerActor :type "Actor Object Reference") (DeltaSeconds :type "Float (single-precision)"))
  (bind _returnvalue (`Actor.K2_GetActorLocation` (`Controller.K2_GetPawn` (`self.AIControllerRef`))))
  (if (not (!= (`self.AIControllerRef`) null))
    (bind _ascharacter_aicontroller (cast `/Game/Blueprints/CharacterAI/CharacterAIController` OwnerActor))
    (set `self.AIControllerRef` _ascharacter_aicontroller))
  (bind _outactors (`GameplayStatics.GetAllActorsOfClass` "/Game/Blueprints/CharacterAI.CharacterAI_C"))
  (set `self.AILocation` _returnvalue)
  (bind _outhits (`KismetSystemLibrary.SphereTraceMultiForObjects` _returnvalue (+ _returnvalue (0.0 0.0 15.0)) 1500.0 (`self.DesiredObjectTypes`) false _outactors))
  (for _array_element _outhits
    (bind (_bblockinghit _binitialoverlap _time _location _impactpoint _normal _impactnormal _physmat _hitactor) (`GameplayStatics.BreakHitResult` _array_element))
    (bind _outhit (`KismetSystemLibrary.LineTraceSingle` (`self.AILocation`) (`Actor.K2_GetActorLocation` _hitactor) "TraceTypeQuery2" false _outactors))
    (bind (_bblockinghit_2 _binitialoverlap_2 _time_2 _location_2 _impactpoint_2 _normal_2 _impactnormal_2 _physmat_2 _hitactor_2) (`GameplayStatics.BreakHitResult` _outhit))
    (if (== _hitactor_2 _hitactor)
      (`BTFunctionLibrary.SetBlackboardValueAsObject` (`self.AITarget`) _hitactor_2)
      (`BTFunctionLibrary.SetBlackboardValueAsVector` (`self.AILocationTarget`) (`Actor.K2_GetActorLocation` _hitactor_2))
      (else
        (`BTFunctionLibrary.SetBlackboardValueAsObject` (`self.AITarget`))))))