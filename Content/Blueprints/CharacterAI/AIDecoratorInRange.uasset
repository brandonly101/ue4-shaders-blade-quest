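; AI behavior tree decorator that passes when the controlled pawn is within detection range of its target.
; It casts the owner to CharacterAIController, caches it, and compares the pawn's distance to the AITarget blackboard actor against RangeDetect.
; An older vector-length comparison with the opposite sense remains unconnected in the graph.
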(fn `PerformConditionCheck`
  (params (OwnerActor :type "Actor Object Reference"))
  (returns (ReturnValue :type Boolean))
  (bind _ascharacter_aicontroller (cast `/Game/Blueprints/CharacterAI/CharacterAIController` OwnerActor))
  (set `self.AIControllerRef` _ascharacter_aicontroller)
  (return (<= (`Actor.GetDistanceTo` (`Controller.K2_GetPawn` (`self.AIControllerRef`)) (`BTFunctionLibrary.GetBlackboardValueAsActor` (`self.AITarget`))) (`self.RangeDetect`))))