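; AI-controlled enemy character with a sword and a floating health and stamina HUD.
; The construction script attaches the sword to the mesh's weapon socket, and its collider applies damage on overlap, gated by attack flags to one hit until reset.
; Tick yaws the HUD's scene component toward the player, pushes health and stamina into the widget, and destroys the actor once it is no longer alive.
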(event `self.ReceiveBeginPlay`)

(event `self.ReceiveActorBeginOverlap`
  (params (OtherActor :type "Actor Object Reference")))

(event `self.SwordCollider.OnComponentBeginOverlap`
  (params (OtherActor :type "Actor Object Reference") (OtherComp :type "PrimitiveComponent Object Reference") (OtherBodyIndex :type Integer) (bFromSweep :type Boolean) (SweepResult :type "HitResult Structure (by ref)"))
  ;[1 1 1] Attack/Damage Logic
  (if (and (`self.isAttacking`) (not (`self.dealtDamage`)) (!= OtherActor self) (`self.canDamage`))
    (bind _returnvalue (`AIBlueprintHelperLibrary.GetAIController` (`self.GetOwner`)))
    (`GameplayStatics.ApplyDamage` OtherActor (`self.Damage`) _returnvalue)
    (set `self.dealtDamage` true)))

(event `self.ReceiveTick`
  (params (DeltaSeconds :type "Float (single-precision)"))
  ;[1 1 1] Enemy HUD
  (`parent.ReceiveTick` DeltaSeconds)
  (`SceneComponent.K2_SetWorldRotation` (`self.Scene`) (`KismetMathLibrary.MakeRot` 0.0 (.yaw (`KismetMathLibrary.FindLookAtRotation` (`SceneComponent.K2_GetComponentLocation` (`self.Scene`)) (`self.K2_GetActorLocation` (`GameplayStatics.GetPlayerCharacter` 0))))) false)
  (bind _asaihud (cast `/Game/Blueprints/AIHUD` (`WidgetComponent.GetUserWidgetObject` (`self.HUD`))))
  (set `/Game/Blueprints/AIHUD.HealthValue` (`self.Health`) _asaihud)
  (set `/Game/Blueprints/AIHUD.StaminaValue` (`self.Stamina`) _asaihud)
  (if (not (`self.isAlive`))
    (`/Engine/EditorBlueprintResources/StandardMacros.DoOnce` false
      (:`Completed`
        (`self.K2_DestroyActor`)))))

(fn `UserConstructionScript`
  (`SceneComponent.K2_AttachTo` (`self.Sword`) (`self.Mesh`) "WEAPON" "KeepRelativeOffset" true))