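; ActivityProtest is an activity Blueprint labeled "Protest the Autocracy" that shows a subtitle when the player's activity begins.
; BeginPlay sets the activity text, and BeginActivity adds a DisplaySubtitle widget, clears ActivityInProgress, then removes all widgets after a short delay.
; An overlap check and a random MultiGate lead into the same subtitle logic but are unconnected and never run.
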(event `self.ReceiveBeginPlay`
  (set `self.TextActivity` "Protest the Autocracy"))

(event `BeginActivity`
  (bind _returnvalue (`|CreateWidget` "/Game/Blueprints/DisplaySubtitle.DisplaySubtitle_C"))
  (`UserWidget.AddToViewport` _returnvalue 0)
  (set `self.ActivityInProgress` false)
  (`KismetSystemLibrary.Delay` 4.0)
  (`WidgetLayoutLibrary.RemoveAllWidgets`))

(fn `UserConstructionScript`
  (`parent.UserConstructionScript`))