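; Activity is an interactable trigger actor that prompts and starts an activity, with an empty BeginActivity event as the apparent hook for specific behavior.
; Any actor overlap creates a DisplayPrompt widget showing TextActivity and sets ActivityOverlap; ending overlap clears all widgets and the flag.
; It enables player input on BeginPlay, so the Activity input action calls BeginActivity only while that flag is set.
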(event `self.ReceiveBeginPlay`
  ;[1 1 1] Enable Input
  (`self.EnableInput` (`GameplayStatics.GetPlayerController` 0)))

(event `self.ReceiveActorBeginOverlap`
  (params (OtherActor :type "Actor Object Reference"))
  ;[1 1 1] Collision Triggers
  (if true
    (bind _returnvalue (`|CreateWidget` "/Game/Blueprints/DisplayPrompt.DisplayPrompt_C" (`GameplayStatics.GetPlayerController` 0)))
    (set `/Game/Blueprints/DisplayPrompt.Activities` (`self.TextActivity`) _returnvalue)
    (`UserWidget.AddToViewport` _returnvalue 0)
    (set `self.ActivityOverlap` true)))

(event `self.ReceiveActorEndOverlap`
  (params (OtherActor :type "Actor Object Reference"))
  ;[1 1 1] Collision Triggers
  (if true
    (`WidgetLayoutLibrary.RemoveAllWidgets`)
    (set `self.ActivityOverlap` false)))

(event `InputAction|Activity`
  ;[1 1 1] Trigger the Activity
  (:`Pressed`
    (if (`self.ActivityOverlap`)
      (`self.Begin Activity`))))

(event `Begin Activity`)

(fn `UserConstructionScript`)